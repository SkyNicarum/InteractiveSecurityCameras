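; BP_SecurityMonitor is an in-game security monitor that displays the live feed of linked security cameras on its screen.
; Shortly after BeginPlay it creates a dynamic screen material and feeds it a render target from the first camera's scene capture, sized by viewport and camera quality.
; SwapCamera detaches the current capture and cycles to the next camera with a new render target.
; NewPlayerInput forwards player input to rotate the active camera.
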(event `self.ReceiveBeginPlay`
  (bind (_returnvalue_x _returnvalue_y) (`KismetMathLibrary.BreakVector2D` (`WidgetLayoutLibrary.GetViewportSize`)))
  (bind _cameraqualitylevel (`/Game/BP_SecurityCamera.CameraQualityLevel` (`|GetArrayItem` (`self.LinkedCamera`))))
  (`KismetSystemLibrary.Delay` 0.1)
  (`/Engine/EditorBlueprintResources/StandardMacros.IsValid` (`|GetArrayItem` (`self.LinkedCamera`))
    (:`Is Valid`
      (bind _returnvalue (`KismetMaterialLibrary.CreateDynamicMaterialInstance` "/Game/M_SecurityCamera.M_SecurityCamera"))
      (bind _output_get (set `self.MatCamera` _returnvalue))
      (`PrimitiveComponent.SetMaterial` (`self.Monitor`) 0 _output_get)
      (bind _returnvalue_2 (`KismetRenderingLibrary.CreateRenderTarget2D` (`KismetMathLibrary.FTrunc` (* _returnvalue_x _cameraqualitylevel)) (`KismetMathLibrary.FTrunc` (* _returnvalue_y _cameraqualitylevel))))
      (bind _output_get_2 (set `self.RTCamera` _returnvalue_2))
      (bind _output_get_3 (set `SceneCaptureComponent2D.TextureTarget` _output_get_2 (`/Game/BP_SecurityCamera.SceneCaptureComponent2D` (`|GetArrayItem` (`self.LinkedCamera`)))))
      (`MaterialInstanceDynamic.SetTextureParameterValue` (`self.MatCamera`) "Texture" _output_get_3)
      (`MaterialInstanceDynamic.SetScalarParameterValue` (`self.MatCamera`) "ScreenBright" (`self.ScreenBright`)))))

(event `SwapCamera`
  (bind (_returnvalue_x _returnvalue_y) (`KismetMathLibrary.BreakVector2D` (`WidgetLayoutLibrary.GetViewportSize`)))
  (bind _cameraqualitylevel (`/Game/BP_SecurityCamera.CameraQualityLevel` (`|GetArrayItem` (`self.LinkedCamera`) (`self.CurrentCamera`))))
  (set `SceneCaptureComponent2D.TextureTarget` null (`/Game/BP_SecurityCamera.SceneCaptureComponent2D` (`|GetArrayItem` (`self.LinkedCamera`) (`self.CurrentCamera`))))
  (`/Engine/EditorBlueprintResources/StandardMacros.IncrementInt` (`self.CurrentCamera`)
    (:`  `
      (if (>= (`self.CurrentCamera`) (`KismetArrayLibrary.Array_Length` (`self.LinkedCamera`)))
        (set `self.CurrentCamera` 0))
      (bind _returnvalue (`KismetRenderingLibrary.CreateRenderTarget2D` (`KismetMathLibrary.FTrunc` (* _returnvalue_x _cameraqualitylevel)) (`KismetMathLibrary.FTrunc` (* _returnvalue_y _cameraqualitylevel))))
      (bind _output_get (set `self.RTCamera` _returnvalue))
      (bind _output_get_2 (set `SceneCaptureComponent2D.TextureTarget` _output_get (`/Game/BP_SecurityCamera.SceneCaptureComponent2D` (`|GetArrayItem` (`self.LinkedCamera`) (`self.CurrentCamera`)))))
      (`MaterialInstanceDynamic.SetTextureParameterValue` (`self.MatCamera`) "Texture" _output_get_2)
      (`MaterialInstanceDynamic.SetScalarParameterValue` (`self.MatCamera`) "ScreenBright" (`self.ScreenBright`)))))

(event `NewPlayerInput`
  (params (HorizontalInput :type "Float (double-precision)") (VerticalInput :type "Float (double-precision)"))
  (`/Game/BP_SecurityCamera.RotateCamera` (`|GetArrayItem` (`self.LinkedCamera`) (`self.CurrentCamera`)) HorizontalInput VerticalInput))

(fn `UserConstructionScript`)